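; BP_ThreadCube is a colored cube actor that shows a countdown of its remaining lifetime and then destroys itself.
; InitBP receives a CubeInfo, uses its Age for the actor's life span and initial text, and applies its Color through a dynamic material instance's CubeColor parameter.
; A looping one-second timer calls SetLiveTimeText to decrement the seconds and refresh the text, so Tick is unused.
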(event `self.InitBP`
  (params (CubeInfo :type "CubeInfo Structure"))
  (bind _output_get (set `self.SecondsToDestroy` CubeInfo_Age))
  (`self.SetLifeSpan` _output_get)
  (`TextRenderComponent.K2_SetText` (`self.AgeText`) (`KismetTextLibrary.Conv_DoubleToText` CubeInfo_Age "HalfToEven"))
  (bind _returnvalue (`PrimitiveComponent.CreateDynamicMaterialInstance` (`self.Cube`) 0 null "None"))
  (`MaterialInstanceDynamic.SetVectorParameterValue` _returnvalue "CubeColor" CubeInfo_Color)
  (`KismetSystemLibrary.K2_SetTimer` null "SetLiveTimeText" 1.0 true))

(fn `SetLiveTimeText`
  (bind _output_get (set `self.SecondsToDestroy` (- (`self.SecondsToDestroy`) 1.0)))
  (`TextRenderComponent.K2_SetText` (`self.AgeText`) (`KismetTextLibrary.Conv_DoubleToText` _output_get "HalfToEven")))

(fn `UserConstructionScript`)